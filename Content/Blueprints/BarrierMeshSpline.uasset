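; Barrier spline actor that lays repeated copies of a mesh along a spline in the construction script, with collision enabled.
; Section step is the mesh's bounding-box length on the chosen forward axis plus Spacing.
; Each step adds a spline mesh component at that distance, combining MeshRotation with the spline rotation.
; Start/end points and tangents are never set, so sections do not bend to follow the curve.
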(fn `UserConstructionScript`
  (bind _spline (`self.Spline`))
  (bind (_returnvalue_min _returnvalue_max) (break `Box` (`StaticMesh.GetBoundingBox` (`self.Spline Mesh`))))
  (bind _returnvalue (* (`self.Index`) (`self.sectionLength`)))
  (bind (_returnvalue_x _returnvalue_y _returnvalue_z) (`KismetMathLibrary.BreakVector` (- _returnvalue_max _returnvalue_min)))
  (if (`|EnumEquality` (`self.In Forward Axis`) "X")
    (set `self.MeshLength` _returnvalue_x)
    (elif (`|EnumEquality` (`self.In Forward Axis`) "Y")
      (set `self.MeshLength` _returnvalue_y)
      (else
        (set `self.MeshLength` _returnvalue_z))))
  (set `self.sectionLength` (+ (`self.Spacing`) (`self.MeshLength`)))
  (for _index (range (+ (`KismetMathLibrary.FTrunc` (/ (`SplineComponent.GetSplineLength` (`self.Spline`)) (`self.sectionLength`))) 1))
    (set `self.Index` _index)
    (bind _returnvalue_2 (`AddComponent|NODE_AddSplineMeshComponent-0` :`RelativeTransform` (`KismetMathLibrary.MakeTransform` (`SplineComponent.GetLocationAtDistanceAlongSpline` _spline _returnvalue "Local") (`KismetMathLibrary.ComposeRotators` (`self.MeshRotation`) (`SplineComponent.GetRotationAtDistanceAlongSpline` _spline _returnvalue "Local")))))
    (`StaticMeshComponent.SetStaticMesh` _returnvalue_2 (`self.Spline Mesh`))
    (`PrimitiveComponent.SetCollisionEnabled` _returnvalue_2 "QueryAndPhysics")
    (`SplineMeshComponent.SetForwardAxis` _returnvalue_2 (`self.In Forward Axis`) true)))