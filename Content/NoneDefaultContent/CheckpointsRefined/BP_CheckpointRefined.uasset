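; BP_CheckpointRefined is a numbered checkpoint trigger that tracks a vehicle's progress through an ordered sequence.
; On box overlap, a BP_Vehicle's CurrentCheckpointRefined advances to this checkpoint's number only if it holds the preceding number, enforcing order.
; The construction script auto-numbers a checkpoint left at zero by looping over all checkpoint actors, ending with their total count.
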(event `self.Box.OnComponentBeginOverlap`
  (params (OverlappedComponent :type "PrimitiveComponent Object Reference") (OtherActor :type "Actor Object Reference") (OtherComp :type "PrimitiveComponent Object Reference") (OtherBodyIndex :type Integer) (bFromSweep :type Boolean) (SweepResult :type "HitResult Structure (by ref)"))
  (bind _checkpointnumber (`self.CheckpointNumber`))
  (bind _asbp_vehicle (cast `/Game/NoneDefaultContent/VehicleStuff/BP_Vehicle` OtherActor))
  (if (== (- _checkpointnumber 1) (`/Game/NoneDefaultContent/VehicleStuff/BP_Vehicle.CurrentCheckpointRefined` _asbp_vehicle))
    (set `/Game/NoneDefaultContent/VehicleStuff/BP_Vehicle.CurrentCheckpointRefined` _checkpointnumber _asbp_vehicle)))

(fn `UserConstructionScript`
  (if (== (`self.CheckpointNumber`) 0)
    (bind _outactors (`GameplayStatics.GetAllActorsOfClass` "BP_CheckpointRefined_C"))
    (for (_ _array_index) _outactors
      (set `self.CheckpointNumber` (+ _array_index 1)))))