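; Porsche vehicle Blueprint that adds speed-reactive exhaust effects on top of its parent class's behavior.
; Each tick, it maps CurrentSpeed to an inverted, clamped factor that is full at standstill and fades to zero as speed rises.
; That factor feeds the Velocity float variable on four left and right exhaust effect components.
; BeginPlay and the construction script only call their parent versions.
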(event `self.ReceiveBeginPlay`
  (`parent.ReceiveBeginPlay`))

(event `self.ReceiveTick`
  (params (DeltaSeconds :type "Float (single-precision)"))
  (`parent.ReceiveTick` DeltaSeconds)
  (`NiagaraComponent.SetVariableFloat` (`self.L_Exhaust`) "Velocity" (`KismetMathLibrary.FClamp` (* (- (/ (`self.CurrentSpeed`) 25.0) 1.0) -1.0)))
  (`NiagaraComponent.SetVariableFloat` (`self.R_Exhaust`) "Velocity" (`KismetMathLibrary.FClamp` (* (- (/ (`self.CurrentSpeed`) 25.0) 1.0) -1.0)))
  (`NiagaraComponent.SetVariableFloat` (`self.R_Exhaust1`) "Velocity" (`KismetMathLibrary.FClamp` (* (- (/ (`self.CurrentSpeed`) 25.0) 1.0) -1.0)))
  (`NiagaraComponent.SetVariableFloat` (`self.L_Exhaust1`) "Velocity" (`KismetMathLibrary.FClamp` (* (- (/ (`self.CurrentSpeed`) 25.0) 1.0) -1.0))))

(fn `UserConstructionScript`
  (`parent.UserConstructionScript`))