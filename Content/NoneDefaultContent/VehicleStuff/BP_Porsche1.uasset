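; Drivable Porsche car Blueprint with keyboard and wheel steering, recolourable body and an orbit camera.
; Each tick the CarForces component simulates physics from throttle and brake input, feeding wheel loads and velocities to RunSimulationFrame.
; Steering weakens with speed and smoothly turns the front wheels, with slight rear counter-steer.
; It also spins tire meshes, widens FOV with speed, auto-recentres the camera and resets speed when a crash stalls the body.
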(event `self.ReceiveBeginPlay`
  ;[1 1 1] Initialisation
  (set `self.RimCompArray` (`|MakeArray` (`self.RR_RimMesh`) (`self.RL_RimMesh`) (`self.FL_RimMesh`) (`self.FR_RimMesh`)))
  (bind _returnvalue (`PrimitiveComponent.CreateDynamicMaterialInstance` (`self.CarBody`) 18 "/Game/NoneDefaultContent/VehicleStuff/M_Car2.M_Car2" "None"))
  (`PrimitiveComponent.SetMaterial` (`self.CarBody`) 18 _returnvalue)
  (set `self.CarColour` _returnvalue)
  (`self.SetCarColour` (struct)))

(event `self.ReceiveTick`
  (params (DeltaSeconds :type "Float (single-precision)"))
  (bind _carforces (`self.CarForces`))
  (bind _carforces_2 (`self.CarForces`))
  ;[1 1 1 1 25] Perform the simulation Calculations
  (`self.UpdateCameraTracking` DeltaSeconds)
  (`CarForcesComponent.PerformSimulationFrame` (`self.CarForces`) DeltaSeconds)
  (`self.ApplyTurning`)
  (`self.RunSimulationFrame` (`.load` (break `TireInfo` (`CarForcesComponent.tireRR` _carforces_2))) (`.load` (break `TireInfo` (`CarForcesComponent.tireRL` _carforces_2))) (`.load` (break `TireInfo` (`CarForcesComponent.tireFR` _carforces_2))) (`.load` (break `TireInfo` (`CarForcesComponent.tireFL` _carforces_2))) (`CarForcesComponent.carVelocity` _carforces_2) (`CarForcesComponent.carAngularVelocity` _carforces_2))
  ;[1 1 1 1 25] Update variables
  (`self.SpinWheels`)
  (set `self.RPMs` (`.engineRPM` (break `EngineInfo` (`CarForcesComponent.engineInfo` _carforces))))
  (set `self.CurrentSpeed` (* (`KismetMathLibrary.VSize` (`CarForcesComponent.carVelocity` _carforces)) 2.23694))
  (`self.CheckForCarCrash`))

(event `EnhancedInput|/Game/DefaultContent/VehicleTemplate/Input/Actions/IA_Throttle`
  (params (ActionValue :type "Float (double-precision)") (ElapsedSeconds :type "Float (double-precision)") (TriggeredSeconds :type "Float (double-precision)") (InputAction :type "InputAction Object Reference" :default "/Game/DefaultContent/VehicleTemplate/Input/Actions/IA_Throttle.IA_Throttle"))
  ;[1 1 1] Set Throttle input
  (:`Started`
    (set `CarForcesComponent.throttleInput` 1.0 (`self.CarForces`)))
  (:`Completed`
    (set `CarForcesComponent.throttleInput` 0.0 (`self.CarForces`))))

(event `FOVChanges`
  (bind _targetfov (`self.targetFOV`))
  (bind _returnvalue (+ (`CameraComponent.FieldOfView` (`self.Camera`)) (* (`GameplayStatics.GetWorldDeltaSeconds`) (`KismetMathLibrary.SignOfFloat` (- _targetfov (`CameraComponent.FieldOfView` (`self.Camera`)))) 7.5)))
  ;[1 1 1] Smoothed FOV changing
  (if (>= (- (`self.targetFOV`) (`CameraComponent.FieldOfView` (`self.Camera`))) 0.0)
    (if (!= (`CameraComponent.FieldOfView` (`self.Camera`)) _targetfov)
      (`CameraComponent.SetFieldOfView` (`self.Camera`) (`KismetMathLibrary.FClamp` _returnvalue 90.0 (`self.targetFOV`))))
    (elif (!= (`CameraComponent.FieldOfView` (`self.Camera`)) (`self.targetFOV`))
      (`CameraComponent.SetFieldOfView` (`self.Camera`) (`KismetMathLibrary.FClamp` _returnvalue 90.0 (`CameraComponent.FieldOfView` (`self.Camera`)))))))

(event `EnhancedInput|/Game/DefaultContent/VehicleTemplate/Input/Actions/IA_Brake`
  (params (ActionValue :type "Float (double-precision)") (ElapsedSeconds :type "Float (double-precision)") (TriggeredSeconds :type "Float (double-precision)") (InputAction :type "InputAction Object Reference" :default "/Game/DefaultContent/VehicleTemplate/Input/Actions/IA_Brake.IA_Brake"))
  ;[1 1 1] Braking
  (:`Started`
    (set `CarForcesComponent.brakeInput` 1.0 (`self.CarForces`)))
  (:`Completed`
    (set `CarForcesComponent.brakeInput` 0.0 (`self.CarForces`))))

(event `SmoothedFrontTireRotations`
  (params (TargetAngle :type "Float (double-precision)"))
  (bind _yaw (.yaw (`SceneComponent.RelativeRotation` (`self.FL_SuspensionMount`))))
  (bind _returnvalue (+ (* (`GameplayStatics.GetWorldDeltaSeconds`) (`KismetMathLibrary.SignOfFloat` (- TargetAngle _yaw)) 75.0) _yaw))
  (bind _returnvalue_2 (`KismetMathLibrary.MakeRotator` 0.0 0.0 (`KismetMathLibrary.FClamp` _returnvalue _yaw TargetAngle)))
  (bind _returnvalue_3 (`KismetMathLibrary.MakeRotator` 0.0 0.0 (`KismetMathLibrary.FClamp` _returnvalue TargetAngle _yaw)))
  ;[1 1 1] Smoothed Wheel Rotation changing
  (if (>= (- TargetAngle (.yaw (`SceneComponent.RelativeRotation` (`self.FL_SuspensionMount`)))) 0.0)
    (`SceneComponent.K2_SetRelativeRotation` (`self.FL_SuspensionMount`) _returnvalue_2 false false)
    (`SceneComponent.K2_SetRelativeRotation` (`self.FR_SuspensionMount`) _returnvalue_2 false false)
    (else
      (`SceneComponent.K2_SetRelativeRotation` (`self.FL_SuspensionMount`) _returnvalue_3 false false)
      (`SceneComponent.K2_SetRelativeRotation` (`self.FR_SuspensionMount`) _returnvalue_3 false false))))

(event `EnhancedInput|/Game/DefaultContent/VehicleTemplate/Input/Actions/IA_TurnRight`
  (params (ActionValue :type "Float (double-precision)") (ElapsedSeconds :type "Float (double-precision)") (TriggeredSeconds :type "Float (double-precision)") (InputAction :type "InputAction Object Reference" :default "/Game/DefaultContent/VehicleTemplate/Input/Actions/IA_TurnRight.IA_TurnRight"))
  ;[1 1 1] Keyboard Turning inputs. Right is +1 and left is -1
  (:`Started`
    (set `self.TurningMultiplier` (+ (`self.TurningMultiplier`) ActionValue))
    (`self.ApplyTurning` :!label _label))
  (:`Completed`
    (set `self.TurningMultiplier` (+ (`self.TurningMultiplier`) -1.0))
    (goto _label)))

(event `EnhancedInput|/Game/DefaultContent/VehicleTemplate/Input/Actions/IA_Steering`
  (params (ActionValue :type "Float (double-precision)") (ElapsedSeconds :type "Float (double-precision)") (TriggeredSeconds :type "Float (double-precision)") (InputAction :type "InputAction Object Reference" :default "/Game/DefaultContent/VehicleTemplate/Input/Actions/IA_Steering.IA_Steering"))
  ;[1 1 1] Wheel turning input
  (:`Triggered`
    (set `self.TurningMultiplier` ActionValue)
    (`self.ApplyTurning`)))

(event `EnhancedInput|/Game/DefaultContent/VehicleTemplate/Input/Actions/IA_TurnLeft`
  (params (ActionValue :type "Float (double-precision)") (ElapsedSeconds :type "Float (double-precision)") (TriggeredSeconds :type "Float (double-precision)") (InputAction :type "InputAction Object Reference" :default "/Game/DefaultContent/VehicleTemplate/Input/Actions/IA_TurnLeft.IA_TurnLeft"))
  ;[1 1 1] Keyboard Turning inputs. Right is +1 and left is -1
  (:`Started`
    (set `self.TurningMultiplier` (+ (`self.TurningMultiplier`) ActionValue))
    (`self.ApplyTurning` :!label _label_2))
  (:`Completed`
    (set `self.TurningMultiplier` (+ (`self.TurningMultiplier`) 1.0))
    (goto _label_2)))

(event `EnhancedInput|/Game/DefaultContent/VehicleTemplate/Input/Actions/IA_CameraLook`
  (params (ActionValue :type "Vector2D Structure") (ElapsedSeconds :type "Float (double-precision)") (TriggeredSeconds :type "Float (double-precision)") (InputAction :type "InputAction Object Reference" :default "/Game/DefaultContent/VehicleTemplate/Input/Actions/IA_CameraLook.IA_CameraLook"))
  (bind (_x _y) (`KismetMathLibrary.BreakVector2D` ActionValue))
  ;[1 1 1] Camera rotation input
  (:`Triggered`
    (set `self.CameraResetTimer` 0.0)
    (`SceneComponent.K2_SetWorldRotation` (`self.SpringArm`) (`KismetMathLibrary.MakeRotator` 0.0 (`KismetMathLibrary.FClamp` (+ _y (.pitch (`SceneComponent.K2_GetComponentRotation` (`self.SpringArm`)))) -70.0 10.0) (+ (.yaw (`SceneComponent.K2_GetComponentRotation` (`self.SpringArm`))) _x)) false false)))

(event `SmoothedRearTireRotations`
  (params (TargetAngle :type "Float (double-precision)"))
  (bind _yaw (.yaw (`SceneComponent.RelativeRotation` (`self.RR_SuspensionMount`))))
  (bind _returnvalue (+ (* (`GameplayStatics.GetWorldDeltaSeconds`) (`KismetMathLibrary.SignOfFloat` (- TargetAngle _yaw)) 75.0) _yaw))
  (bind _returnvalue_2 (`KismetMathLibrary.MakeRotator` 0.0 0.0 (`KismetMathLibrary.FClamp` _returnvalue TargetAngle _yaw)))
  (bind _returnvalue_3 (`KismetMathLibrary.MakeRotator` 0.0 0.0 (`KismetMathLibrary.FClamp` _returnvalue _yaw TargetAngle)))
  ;[1 1 1] Smoothed Wheel Rotation changing
  (if (>= (- TargetAngle (.yaw (`SceneComponent.RelativeRotation` (`self.RR_SuspensionMount`)))) 0.0)
    (`SceneComponent.K2_SetRelativeRotation` (`self.RL_SuspensionMount`) _returnvalue_3 false false)
    (`SceneComponent.K2_SetRelativeRotation` (`self.RR_SuspensionMount`) _returnvalue_3 false false)
    (else
      (`SceneComponent.K2_SetRelativeRotation` (`self.RL_SuspensionMount`) _returnvalue_2 false false)
      (`SceneComponent.K2_SetRelativeRotation` (`self.RR_SuspensionMount`) _returnvalue_2 false false))))

(fn `ApplyTurning`
  (locals (TurningAngle :type "Float (double-precision)"))
  (`|ExecutionSequence`
    (:`then_0`
      ;[1 1 1] Set the delta
      (`|VariableSetRef` (`.delta` (break `TireInfo` (`CarForcesComponent.tireFR` (`self.CarForces`)))) (* (`self.TurningMultiplier`) 50.0 (`KismetMathLibrary.FClamp` (`KismetMathLibrary.MultiplyMultiply_FloatFloat` (- 1.0 (/ (`self.CurrentSpeed`) 215.0)) 3.32193) 0.1))))
    (:`then_1`
      ;[1 1 1] Set the Turning Angle
      (set `local.TurningAngle` (`KismetMathLibrary.FClamp` (`.delta` (break `TireInfo` (`CarForcesComponent.tireFR` (`self.CarForces`)))) -30.0 30.0)))
    (:`then_2`
      ;[1 1 1] Turn the front wheels
      (`self.SmoothedFrontTireRotations` (`local.TurningAngle`))
      (`self.SmoothedRearTireRotations` (* (`local.TurningAngle`) -0.0675)))))

(fn `CheckForCarCrash`
  (if (>= (`KismetMathLibrary.Abs` (.x (`CarForcesComponent.carVelocity` (`self.CarForces`)))) 2.0)
    (if (<= (`KismetMathLibrary.VSize` (`SceneComponent.GetComponentVelocity` (`self.CarBody`))) 40.0)
      (bind _output_get (set `self.CrashTimer` (+ (`self.CrashTimer`) (`GameplayStatics.GetWorldDeltaSeconds`))))
      (if (> _output_get 0.1)
        (`CarForcesComponent.ResetCarSpeed` (`self.CarForces`)))
      (else
        (set `self.CrashTimer` 0.0)))))

(fn `PrintDebuggingInfo`
  (bind _carforces (`self.CarForces`))
  (bind _carforces_2 (`self.CarForces`))
  (bind _carforces_3 (`self.CarForces`))
  (bind _carforces_4 (`self.CarForces`))
  (bind (_engineangularvelocity _enginerpm _enginemaxtorque _enginemintorque _currenttorque _currentgear _drivingtorqueperwheel) (break `EngineInfo` (`CarForcesComponent.engineInfo` _carforces_3)))
  (`KismetSystemLibrary.PrintString` (`KismetStringLibrary.Concat_StrStr` "Velocity: " (`KismetStringLibrary.Conv_VectorToString` (`CarForcesComponent.carVelocity` _carforces_3))) true false (struct :`R` 1.0 :`G` 0.030497 :`B` 0.06698 :`A` 1.0) 2.0 "0")
  (`KismetSystemLibrary.PrintString` (`KismetStringLibrary.Concat_StrStr` "Acceleration: " (`KismetStringLibrary.Conv_VectorToString` (`CarForcesComponent.carAcceleration` _carforces_3)) " \n") true false (struct :`R` 1.0 :`G` 0.030497 :`B` 0.06698 :`A` 1.0) 2.0 "1")
  (`KismetSystemLibrary.PrintString` (`KismetStringLibrary.Concat_StrStr` "Torque per wheel: " (`KismetStringLibrary.Conv_DoubleToString` _drivingtorqueperwheel) "      Engine Speed: " (`KismetStringLibrary.Conv_DoubleToString` _engineangularvelocity) " \nMax Torque: " (`KismetStringLibrary.Conv_DoubleToString` _enginemaxtorque) "     Min Torque: " (`KismetStringLibrary.Conv_DoubleToString` _enginemintorque) " \n") true false (struct :`R` 1.0 :`G` 0.030497 :`B` 0.06698 :`A` 1.0) 2.0 "3")
  (`KismetSystemLibrary.PrintString` (`KismetStringLibrary.Concat_StrStr` "FR Load: " (`KismetStringLibrary.Conv_DoubleToString` (`.load` (break `TireInfo` (`CarForcesComponent.tireFR` _carforces_2)))) "   FL Load: " (`KismetStringLibrary.Conv_DoubleToString` (`.load` (break `TireInfo` (`CarForcesComponent.tireFL` _carforces_2)))) " \nRR Load: " (`KismetStringLibrary.Conv_DoubleToString` (`.load` (break `TireInfo` (`CarForcesComponent.tireRR` _carforces_2)))) "    RL Load: " (`KismetStringLibrary.Conv_DoubleToString` (`.load` (break `TireInfo` (`CarForcesComponent.tireRL` _carforces_2)))) " \nload to weight ratio: " (`KismetStringLibrary.Conv_DoubleToString` (`CarForcesComponent.totalWheelLoadToCarWeightRatio` _carforces_2)) " \n") true false (struct :`R` 1.0 :`G` 0.030497 :`B` 0.06698 :`A` 1.0) 2.0 "4")
  (`KismetSystemLibrary.PrintString` (`KismetStringLibrary.Concat_StrStr` "Throttle: " (`KismetStringLibrary.Conv_DoubleToString` (`CarForcesComponent.throttleInput` _carforces)) "    Clutch: " (`KismetStringLibrary.Conv_DoubleToString` (`CarForcesComponent.clutchInput` _carforces)) "    Brake: " (`KismetStringLibrary.Conv_DoubleToString` (`CarForcesComponent.brakeInput` _carforces))) true false (struct :`R` 1.0 :`G` 0.030497 :`B` 0.06698 :`A` 1.0) 2.0 "5")
  (`KismetSystemLibrary.PrintString` (`KismetStringLibrary.Concat_StrStr` "FR ang vel: " (`KismetStringLibrary.Conv_DoubleToString` (`.angularVelocity` (break `TireInfo` (`CarForcesComponent.tireFR` _carforces_4)))) "     FL ang vel: " (`KismetStringLibrary.Conv_DoubleToString` (`.angularVelocity` (break `TireInfo` (`CarForcesComponent.tireFL` _carforces_4)))) " \nRR ang vel: " (`KismetStringLibrary.Conv_DoubleToString` (`.angularVelocity` (break `TireInfo` (`CarForcesComponent.tireRR` _carforces_4)))) "     RL ang vel: " (`KismetStringLibrary.Conv_DoubleToString` (`.angularVelocity` (break `TireInfo` (`CarForcesComponent.tireRL` _carforces_4))))) true false (struct :`R` 1.0 :`G` 0.030497 :`B` 0.06698 :`A` 1.0) 2.0 "7")
  (`KismetSystemLibrary.PrintString` (`KismetStringLibrary.Concat_StrStr` "Wheel Delta: " (`KismetStringLibrary.Conv_DoubleToString` (`.delta` (break `TireInfo` (`CarForcesComponent.tireFR` (`self.CarForces`)))))) true false (struct :`R` 1.0 :`G` 0.030497 :`B` 0.06698 :`A` 1.0) 2.0 "8"))

(fn `SetCarColour`
  (params (Colour :type "LinearColor Structure") (Metallic :type "Float (double-precision)"))
  (bind _carcolour (`self.CarColour`))
  (`MaterialInstanceDynamic.SetVectorParameterValue` _carcolour "Colour" Colour)
  (`MaterialInstanceDynamic.SetScalarParameterValue` _carcolour "Metallic" Metallic))

(fn `SpinWheels`
  (bind _returnvalue (`KismetMathLibrary.MakeRotator` 0.0 (* (`KismetMathLibrary.DegreesToRadians` (`.angularVelocity` (break `TireInfo` (`CarForcesComponent.tireFR` (`self.CarForces`))))) (`GameplayStatics.GetWorldDeltaSeconds`) -600.0)))
  (`SceneComponent.K2_AddLocalRotation` (`self.FL_TireMesh`) _returnvalue false false)
  (`SceneComponent.K2_AddLocalRotation` (`self.FR_TireMesh`) _returnvalue false false)
  (`SceneComponent.K2_AddLocalRotation` (`self.RL_TireMesh`) _returnvalue false false)
  (`SceneComponent.K2_AddLocalRotation` (`self.RR_TireMesh`) _returnvalue false false))

(fn `UpdateCameraTracking`
  (params (deltaTime :type "Float (double-precision)"))
  (`|ExecutionSequence`
    (:`then_0`
      ;[1 1 1] Camera rotation reset
      (bind _output_get (set `self.CameraResetTimer` (+ (`local.deltaTime`) (`self.CameraResetTimer`))))
      (if (>= _output_get 2.0)
        (`SceneComponent.K2_SetWorldRotation` (`self.SpringArm`) (`KismetMathLibrary.TransformRotation` (`self.GetTransform`) (struct :`Pitch` -10.0)) false false)))
    (:`then_1`
      ;[1 1 1] FOV Change
      (set `self.targetFOV` (+ (/ (`self.CurrentSpeed`) 5.0) 90.0))
      (`self.FOVChanges`))))

(fn `UserConstructionScript`)