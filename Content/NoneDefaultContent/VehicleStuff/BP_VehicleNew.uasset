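; BP_VehicleNew is a vehicle Blueprint that drives a car simulation and provides throttle control.
; Each Tick passes the four tire loads and car velocity from CarForces into RunSimulationFrame, then prints debug output including the CarBody center of mass.
; IA_Throttle steps the clamped throttle input up or down per trigger, independent of delta time, and flips direction each time the input completes.
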(event `self.ReceiveTick`
  (params (DeltaSeconds :type "Float (single-precision)"))
  (bind _carforces (`self.CarForces`))
  (`self.RunSimulationFrame` (`.load` (break `TireInfo` (`CarForcesComponent.tireFR` _carforces))) (`.load` (break `TireInfo` (`CarForcesComponent.tireFL` _carforces))) (`.load` (break `TireInfo` (`CarForcesComponent.tireRR` _carforces))) (`.load` (break `TireInfo` (`CarForcesComponent.tireRL` _carforces))) (`CarForcesComponent.carVelocity` _carforces))
  (`KismetSystemLibrary.PrintString` "Hello" true false (struct :`G` 0.66 :`B` 1.0 :`A` 1.0) 2.0 "1")
  (`KismetSystemLibrary.PrintString` (`KismetStringLibrary.Conv_VectorToString` (`PrimitiveComponent.GetCenterOfMass` (`self.CarBody`) "None")) true true (struct :`G` 0.66 :`B` 1.0 :`A` 1.0) 2.0 "3"))

(event `EnhancedInput|/Game/DefaultContent/VehicleTemplate/Input/Actions/IA_Throttle`
  (params (ActionValue :type "Float (double-precision)") (ElapsedSeconds :type "Float (double-precision)") (TriggeredSeconds :type "Float (double-precision)") (InputAction :type "InputAction Object Reference" :default "/Game/DefaultContent/VehicleTemplate/Input/Actions/IA_Throttle.IA_Throttle"))
  (bind _carforces (`self.CarForces`))
  (bind _carforces_2 (`self.CarForces`))
  (:`Triggered`
    (if (`self.IncreaseThrottle`)
      (bind _output_get (set `CarForcesComponent.throttleInput` (`KismetMathLibrary.FClamp` (+ (`CarForcesComponent.throttleInput` _carforces_2) 0.005)) _carforces_2))
      (`KismetSystemLibrary.PrintString` (`KismetStringLibrary.Conv_DoubleToString` _output_get) true false (struct :`G` 0.66 :`B` 1.0 :`A` 1.0) 2.0 "2")
      (else
        (set `CarForcesComponent.throttleInput` (`KismetMathLibrary.FClamp` (+ (`CarForcesComponent.throttleInput` _carforces) -0.005)) _carforces))))
  (:`Completed`
    (set `self.IncreaseThrottle` (not (`self.IncreaseThrottle`)))))

(fn `UserConstructionScript`)