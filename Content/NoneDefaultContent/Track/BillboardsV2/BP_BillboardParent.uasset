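; Parent Blueprint for track billboards that plays a video on repeat through a Media Player.
; From BeginPlay, a self-calling Loop event opens the Media Source, waits briefly for it to load, then plays it.
; It then delays by the Seconds field of the media's duration before calling itself again, so repetition is timer-driven and reopens the source each cycle.
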(event `self.ReceiveBeginPlay`
  (`self.Loop`))

(event `Loop`
  (bind _mediaplayer (`self.MediaPlayer`))
  (bind (_returnvalue_days _returnvalue_hours _returnvalue_minutes _returnvalue_seconds) (`KismetMathLibrary.BreakTimespan` (`MediaPlayer.GetDuration` _mediaplayer)))
  (`MediaPlayer.OpenSource` _mediaplayer (`self.MediaSource`))
  (`KismetSystemLibrary.Delay` 2.0)
  (`MediaPlayer.Play` _mediaplayer)
  (`KismetSystemLibrary.Delay` (`KismetMathLibrary.Conv_IntToDouble` _returnvalue_seconds))
  (`self.Loop`))

(fn `UserConstructionScript`)