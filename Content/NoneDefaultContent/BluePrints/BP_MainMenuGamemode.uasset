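; Game mode, named for the main menu, that tracks lap timing and per-track best times for Tokyo and Fuji.
; SetTimes loads or creates the save and reads the level's best time; only Fuji also starts the finish line timer and sets the vehicle's lap field.
; EndLapTime resets the current time and saves improved bests, but to slot "Lap08" while loading uses "Lapping".
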(event `SetTimes`
  (bind _returnvalue (`GameplayStatics.GetActorOfClass` "/Game/NoneDefaultContent/CheckpointsRefined/BP_FinishLineRefined.BP_FinishLineRefined_C"))
  (set `self.FinishLineRef` _returnvalue)
  (bind _returnvalue_2 (`GameplayStatics.LoadGameFromSlot` "Lapping"))
  (bind _asbp_save_game (cast `/Game/NoneDefaultContent/CheckpointsRefined/BP_SaveGame` _returnvalue_2)
    (:`then`
      (bind _output_get (set `self.SaveGameRef` _asbp_save_game)))
    (:`CastFailed`
      (bind _returnvalue_3 (`GameplayStatics.CreateSaveGameObject` "/Game/NoneDefaultContent/CheckpointsRefined/BP_SaveGame.BP_SaveGame_C"))
      (bind _output_get_2 (set `self.SaveGameRef` _returnvalue_3))
      (`GameplayStatics.SaveGameToSlot` _output_get_2 "Lapping")))
  (switch `string` (`KismetStringLibrary.Conv_NameToString` (`self.LevelToLoad`))
    (:`TokyoBuildings`
      (set `self.BestLapTime` (`/Game/NoneDefaultContent/CheckpointsRefined/BP_SaveGame.TokyoBestLapTime` _output_get)))
    (:`MainFuji`
      (set `self.BestLapTime` (`/Game/NoneDefaultContent/CheckpointsRefined/BP_SaveGame.FujiBestLapTime` _output_get))
      (`/Game/NoneDefaultContent/CheckpointsRefined/BP_FinishLineRefined.StartLapTime` (`self.FinishLineRef`))
      (bind _asbp_vehicle (cast `/Game/NoneDefaultContent/VehicleStuff/BP_Vehicle` (`GameplayStatics.GetPlayerPawn` 0)))
      (set `/Game/NoneDefaultContent/VehicleStuff/BP_Vehicle.CurrentLapRefined` (`/Game/NoneDefaultContent/CheckpointsRefined/BP_FinishLineRefined.NumberOfLaps` (`self.FinishLineRef`)) _asbp_vehicle))))

(fn `EndLapTime`
  (bind _bestlaptime (`self.BestLapTime`))
  (bind _savegameref (`self.SaveGameRef`))
  (if (< (`self.CurrentLapTime`) (`self.BestLapTime`))
    (set `self.BestLapTime` (`self.CurrentLapTime`))
    (set `self.CurrentLapTime` 0.0)
    (switch `string` (`KismetStringLibrary.Conv_NameToString` (`self.LevelToLoad`))
      (:`TokyoBuildings`
        (set `/Game/NoneDefaultContent/CheckpointsRefined/BP_SaveGame.TokyoBestLapTime` _bestlaptime _savegameref))
      (:`MainFuji`
        (set `/Game/NoneDefaultContent/CheckpointsRefined/BP_SaveGame.FujiBestLapTime` _bestlaptime _savegameref)))
    (`GameplayStatics.SaveGameToSlot` _savegameref "Lap08")
    (else
      (set `self.CurrentLapTime` 0.0))))

(fn `StartLapTime`
  (set `self.bLapStarted` true))

(fn `UserConstructionScript`)