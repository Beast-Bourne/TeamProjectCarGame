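; BP_CheckpointManager tracks progress through the level's BP_Checkpoint actors and supplies the respawn transform.
; InitialiseCheckpoints gathers every checkpoint into an array in the order found, without sorting by CheckpointNumber.
; SetCurrentCheckpoint advances only to the next number in sequence and prints the checkpoint's name.
; GetRespawnLocation indexes the array by current number minus one, returning that root's location and rotation at unit scale.
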(event `InitialiseCheckpoints`
  (bind _outactors (`GameplayStatics.GetAllActorsOfClass` "/Game/NoneDefaultContent/RaceStuff/Checkpoints/BP_Checkpoint.BP_Checkpoint_C"))
  (for _array_element _outactors
    (`KismetArrayLibrary.Array_Add` (`self.CheckpointArray`) _array_element)))

(fn `GetRespawnLocation`
  (returns (RespawnTransform :type "Transform Structure"))
  (bind (_returnvalue_location _returnvalue_rotation) (`KismetMathLibrary.BreakTransform` (`SceneComponent.K2_GetComponentToWorld` (`/Game/NoneDefaultContent/RaceStuff/Checkpoints/BP_Checkpoint.DefaultSceneRoot` (`|GetArrayItem` (`self.CheckpointArray`) (- (`self.CurrentCheckpoint`) 1))))))
  (if (> (`self.CurrentCheckpoint`) 0)
    (return (`KismetMathLibrary.MakeTransform` _returnvalue_location _returnvalue_rotation))))

(fn `SetCurrentCheckpoint`
  (params (Checkpoint :type "/Game/NoneDefaultContent/RaceStuff/Checkpoints/BP_Checkpoint Object Reference"))
  (bind _checkpointnumber (`/Game/NoneDefaultContent/RaceStuff/Checkpoints/BP_Checkpoint.CheckpointNumber` Checkpoint))
  (if (== (- _checkpointnumber 1) (`self.CurrentCheckpoint`))
    (set `self.CurrentCheckpoint` _checkpointnumber)
    (`KismetSystemLibrary.PrintString` (`KismetSystemLibrary.GetObjectName` Checkpoint))))

(fn `UserConstructionScript`)