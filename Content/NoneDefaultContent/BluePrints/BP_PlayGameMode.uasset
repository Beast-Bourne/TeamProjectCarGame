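; BP_PlayGameMode runs race lap timing, storing per-track best times for Tokyo and Fuji in a save game.
; Tick accumulates lap time and prints the best.
; Vehicle overlaps compare checkpoint and lap counts with BP_FinishLineRefined to start laps, end them or quit the game after the last.
; BeginPlay loads or creates the save; on Fuji it also starts timing immediately and puts the vehicle on the final lap.
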(event `self.ReceiveTick`
  (params (DeltaSeconds :type "Float (single-precision)"))
  (`KismetSystemLibrary.PrintString` (`KismetStringLibrary.Conv_DoubleToString` (`self.BestLapTime`)))
  (if (`self.bLapStarted`)
    (set `self.CurrentLapTime` (+ (`self.CurrentLapTime`) (`GameplayStatics.GetWorldDeltaSeconds`)))))

(event `self.ReceiveActorBeginOverlap`
  (params (OtherActor :type "Actor Object Reference"))
  (bind _finishlineref (`self.FinishLineRef`))
  (bind _asbp_vehicle (cast `/Game/NoneDefaultContent/VehicleStuff/BP_Vehicle` OtherActor))
  (set `self.VehicleRef` _asbp_vehicle)
  (if (== (`/Game/NoneDefaultContent/CheckpointsRefined/BP_FinishLineRefined.NumberOfCheckpoints` _finishlineref) (`/Game/NoneDefaultContent/VehicleStuff/BP_Vehicle.CurrentCheckpointRefined` _asbp_vehicle))
    (bind _currentlaprefined (`/Game/NoneDefaultContent/VehicleStuff/BP_Vehicle.CurrentLapRefined` _asbp_vehicle))
    (if (== (`/Game/NoneDefaultContent/CheckpointsRefined/BP_FinishLineRefined.NumberOfLaps` _finishlineref) _currentlaprefined)
      (`self.EndLapTime`)
      (`KismetSystemLibrary.QuitGame` null "Quit")
      (else
        (set `/Game/NoneDefaultContent/VehicleStuff/BP_Vehicle.CurrentLapRefined` (+ _currentlaprefined 1) _asbp_vehicle)
        (set `/Game/NoneDefaultContent/VehicleStuff/BP_Vehicle.CurrentCheckpointRefined` 0 _asbp_vehicle)
        (`self.EndLapTime`)
        (`self.StartLapTime`)))
    (elif (not (`/Game/NoneDefaultContent/VehicleStuff/BP_Vehicle.bIsLapping` _asbp_vehicle))
      (set `/Game/NoneDefaultContent/VehicleStuff/BP_Vehicle.bIsLapping` true _asbp_vehicle)
      (set `/Game/NoneDefaultContent/VehicleStuff/BP_Vehicle.CurrentLapRefined` (+ (`/Game/NoneDefaultContent/VehicleStuff/BP_Vehicle.CurrentLapRefined` _asbp_vehicle) 1) _asbp_vehicle)
      (`self.StartLapTime`))))

(event `self.ReceiveBeginPlay`
  (bind _returnvalue (`GameplayStatics.GetActorOfClass` "/Game/NoneDefaultContent/CheckpointsRefined/BP_FinishLineRefined.BP_FinishLineRefined_C"))
  (set `self.FinishLineRef` _returnvalue)
  (bind _returnvalue_2 (`GameplayStatics.LoadGameFromSlot` "Lap08"))
  (bind _asbp_save_game (cast `/Game/NoneDefaultContent/CheckpointsRefined/BP_SaveGame` _returnvalue_2)
    (:`then`
      (bind _output_get (set `self.SaveGameRef` _asbp_save_game)))
    (:`CastFailed`
      (bind _returnvalue_3 (`GameplayStatics.CreateSaveGameObject` "/Game/NoneDefaultContent/CheckpointsRefined/BP_SaveGame.BP_SaveGame_C"))
      (bind _output_get_2 (set `self.SaveGameRef` _returnvalue_3))
      (`GameplayStatics.SaveGameToSlot` _output_get_2 "Lap08")))
  (switch `string` (`KismetStringLibrary.Conv_NameToString` (`self.LevelToLoad`))
    (:`TokyoBuildings`
      (set `self.BestLapTime` (`/Game/NoneDefaultContent/CheckpointsRefined/BP_SaveGame.TokyoBestLapTime` _output_get)))
    (:`MainFuji`
      (set `self.BestLapTime` (`/Game/NoneDefaultContent/CheckpointsRefined/BP_SaveGame.FujiBestLapTime` _output_get))
      (`self.StartLapTime`)
      (bind _asbp_vehicle (cast `/Game/NoneDefaultContent/VehicleStuff/BP_Vehicle` (`GameplayStatics.GetPlayerPawn` 0)))
      (set `/Game/NoneDefaultContent/VehicleStuff/BP_Vehicle.CurrentLapRefined` (`/Game/NoneDefaultContent/CheckpointsRefined/BP_FinishLineRefined.NumberOfLaps` (`self.FinishLineRef`)) _asbp_vehicle))))

(fn `EndLapTime`
  (bind _bestlaptime (`self.BestLapTime`))
  (bind _savegameref (`self.SaveGameRef`))
  (if (< (`self.CurrentLapTime`) (`self.BestLapTime`))
    (set `self.BestLapTime` (`self.CurrentLapTime`))
    (set `self.CurrentLapTime` 0.0)
    (switch `string` (`KismetStringLibrary.Conv_NameToString` (`self.LevelToLoad`))
      (:`TokyoBuildings`
        (set `/Game/NoneDefaultContent/CheckpointsRefined/BP_SaveGame.TokyoBestLapTime` _bestlaptime _savegameref))
      (:`MainFuji`
        (set `/Game/NoneDefaultContent/CheckpointsRefined/BP_SaveGame.FujiBestLapTime` _bestlaptime _savegameref)))
    (`GameplayStatics.SaveGameToSlot` _savegameref "Lap08")
    (else
      (set `self.CurrentLapTime` 0.0))))

(fn `StartLapTime`
  (set `self.bLapStarted` true))

(fn `UserConstructionScript`)