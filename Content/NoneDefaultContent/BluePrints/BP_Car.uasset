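; BP_Car is a car Blueprint that acts as a test rig for wheel load calculations under varying acceleration, slope and banking.
; Its driving inputs are repurposed as step controls: handbrake/reset change acceleration, steering changes gradient, and throttle/brake change bank angle, with angles held in radians.
; Each press has CarForces recalculate wheel loads, then PrintStuff tilts CarBody to both angles and prints accelerations, angles, load ratio and per-wheel loads.
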(event `EnhancedInput|/Game/VehicleTemplate/Input/Actions/IA_Handbrake`
  (params (ActionValue :type Boolean) (ElapsedSeconds :type "Float (double-precision)") (TriggeredSeconds :type "Float (double-precision)") (InputAction :type "InputAction Object Reference" :default "/Game/VehicleTemplate/Input/Actions/IA_Handbrake.IA_Handbrake"))
  (:`Started`
    (bind _output_get (set `self.Accel` (+ (`self.Accel`) -2.0)))
    (set `CarForcesComponent.longitudinalAcceleration` _output_get (`self.CarForces`))
    (bind _returnvalue (`CarForcesComponent.CalculateWheelLoads` (`self.CarForces`) (`self.BankAngle`) (`self.GradientAngle`) (`self.Accel`)))
    (set `self.Loads` _returnvalue)
    (`self.PrintStuff`)))

(event `EnhancedInput|/Game/VehicleTemplate/Input/Actions/IA_Reset`
  (params (ActionValue :type Boolean) (ElapsedSeconds :type "Float (double-precision)") (TriggeredSeconds :type "Float (double-precision)") (InputAction :type "InputAction Object Reference" :default "/Game/VehicleTemplate/Input/Actions/IA_Reset.IA_Reset"))
  (:`Started`
    (bind _output_get (set `self.Accel` (+ (`self.Accel`) 2.0)))
    (set `CarForcesComponent.longitudinalAcceleration` _output_get (`self.CarForces`))
    (bind _returnvalue (`CarForcesComponent.CalculateWheelLoads` (`self.CarForces`) (`self.BankAngle`) (`self.GradientAngle`) (`self.Accel`)))
    (set `self.Loads` _returnvalue)
    (`self.PrintStuff`)))

(event `EnhancedInput|/Game/VehicleTemplate/Input/Actions/IA_Steering`
  (params (ActionValue :type "Float (double-precision)") (ElapsedSeconds :type "Float (double-precision)") (TriggeredSeconds :type "Float (double-precision)") (InputAction :type "InputAction Object Reference" :default "/Game/VehicleTemplate/Input/Actions/IA_Steering.IA_Steering"))
  (:`Started`
    (if (> ActionValue 0.0)
      (set `self.GradientAngle` (+ (`self.GradientAngle`) (`KismetMathLibrary.DegreesToRadians` 2.0)))
      (else
        (set `self.GradientAngle` (- (`self.GradientAngle`) (`KismetMathLibrary.DegreesToRadians` 2.0)))))
    (bind _returnvalue (`CarForcesComponent.CalculateWheelLoads` (`self.CarForces`) (`self.BankAngle`) (`self.GradientAngle`) (`self.Accel`)))
    (set `self.Loads` _returnvalue)
    (`self.PrintStuff`)))

(event `EnhancedInput|/Game/VehicleTemplate/Input/Actions/IA_Throttle`
  (params (ActionValue :type "Float (double-precision)") (ElapsedSeconds :type "Float (double-precision)") (TriggeredSeconds :type "Float (double-precision)") (InputAction :type "InputAction Object Reference" :default "/Game/VehicleTemplate/Input/Actions/IA_Throttle.IA_Throttle"))
  (:`Started`
    (bind _output_get (set `self.BankAngle` (+ (`self.BankAngle`) (`KismetMathLibrary.DegreesToRadians` 2.0))))
    (bind _returnvalue (`CarForcesComponent.CalculateWheelLoads` (`self.CarForces`) _output_get (`self.GradientAngle`) (`self.Accel`)))
    (set `self.Loads` _returnvalue)
    (`self.PrintStuff`)))

(event `EnhancedInput|/Game/VehicleTemplate/Input/Actions/IA_Brake`
  (params (ActionValue :type "Float (double-precision)") (ElapsedSeconds :type "Float (double-precision)") (TriggeredSeconds :type "Float (double-precision)") (InputAction :type "InputAction Object Reference" :default "/Game/VehicleTemplate/Input/Actions/IA_Brake.IA_Brake"))
  (:`Started`
    (bind _output_get (set `self.BankAngle` (- (`self.BankAngle`) (`KismetMathLibrary.DegreesToRadians` 2.0))))
    (bind _returnvalue (`CarForcesComponent.CalculateWheelLoads` (`self.CarForces`) _output_get (`self.GradientAngle`) (`self.Accel`)))
    (set `self.Loads` _returnvalue)
    (`self.PrintStuff`)))

(event `PrintStuff`
  (bind _returnvalue (`KismetMathLibrary.RadiansToDegrees` (`self.BankAngle`)))
  (bind _returnvalue_2 (`KismetMathLibrary.RadiansToDegrees` (`self.GradientAngle`)))
  (bind (_frontright _frontleft _rearright _rearleft) (break `WheelLoads` (`CarForcesComponent.wheelLoads` (`self.CarForces`))))
  (`KismetSystemLibrary.PrintString` (`KismetStringLibrary.Concat_StrStr` "Wheel load ratio: " (`KismetStringLibrary.Conv_DoubleToString` (`CarForcesComponent.totalWheelLoadToCarWeightRatio` (`self.CarForces`)))) true true (struct :`R` 1.0 :`G` 0.061617 :`A` 1.0) 20.0 "-4")
  (`KismetSystemLibrary.PrintString` (`KismetStringLibrary.Concat_StrStr` "Forward accel: " (`KismetStringLibrary.Conv_DoubleToString` (`CarForcesComponent.longitudinalAcceleration` (`self.CarForces`)))) true true (struct :`R` 1.0 :`G` 0.061246 :`A` 1.0) 20.0 "-3")
  (`KismetSystemLibrary.PrintString` (`KismetStringLibrary.Concat_StrStr` "Centripetal accel: " (`KismetStringLibrary.Conv_DoubleToString` (`CarForcesComponent.lateralAcceleration` (`self.CarForces`)))) true true (struct :`R` 1.0 :`G` 0.061246 :`A` 1.0) 20.0 "-2")
  (`SceneComponent.K2_SetWorldRotation` (`self.CarBody`) (`KismetMathLibrary.MakeRotator` _returnvalue _returnvalue_2) false false)
  (`KismetSystemLibrary.PrintString` (`KismetStringLibrary.Concat_StrStr` "Gradient Angle: " (`KismetStringLibrary.Conv_DoubleToString` _returnvalue_2)) true true (struct :`R` 1.0 :`G` 0.061246 :`A` 1.0) 20.0 "-1")
  (`KismetSystemLibrary.PrintString` (`KismetStringLibrary.Concat_StrStr` "Banked Angle: " (`KismetStringLibrary.Conv_DoubleToString` _returnvalue)) true true (struct :`R` 1.0 :`G` 0.061246 :`A` 1.0) 20.0 "0")
  (`KismetSystemLibrary.PrintString` (`KismetStringLibrary.Concat_StrStr` "Front Right: " (`KismetStringLibrary.Conv_DoubleToString` _frontright)) true true (struct :`G` 0.66 :`B` 1.0 :`A` 1.0) 20.0 "1")
  (`KismetSystemLibrary.PrintString` (`KismetStringLibrary.Concat_StrStr` "Front Left: " (`KismetStringLibrary.Conv_DoubleToString` _frontleft)) true true (struct :`G` 0.66 :`B` 1.0 :`A` 1.0) 20.0 "2")
  (`KismetSystemLibrary.PrintString` (`KismetStringLibrary.Concat_StrStr` "Back Right: " (`KismetStringLibrary.Conv_DoubleToString` _rearright)) true true (struct :`G` 0.66 :`B` 1.0 :`A` 1.0) 20.0 "3")
  (`KismetSystemLibrary.PrintString` (`KismetStringLibrary.Concat_StrStr` "Back Left: " (`KismetStringLibrary.Conv_DoubleToString` _rearleft)) true true (struct :`G` 0.66 :`B` 1.0 :`A` 1.0) 20.0 "4"))

(fn `UserConstructionScript`)